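; BP_Projectile is a projectile that destroys enemies and health packs on contact and awards score for enemy kills.
; Sphere overlaps spawn a collision effect on tunnels, or an explosion on enemies, adding five to the BP_Player's UserScore.
; A separate Box overlap explodes health packs without scoring, and the projectile destroys itself in all three cases.
; Sphere hits from non-owner actors make the Sphere ignore the player pawn when moving.
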(event `self.ReceiveTick`
  (params (DeltaSeconds :type "Float (single-precision)")))

(event `self.Sphere.OnComponentBeginOverlap`
  (params (OverlappedComponent :type "PrimitiveComponent Object Reference") (OtherActor :type "Actor Object Reference") (OtherComp :type "PrimitiveComponent Object Reference") (OtherBodyIndex :type Integer) (bFromSweep :type Boolean) (SweepResult :type "HitResult Structure (by ref)"))
  (cast `/Game/InfiniteMatrix/Blueprints/BP_Tunnel` OtherActor
    (:`then`
      (`NiagaraFunctionLibrary.SpawnSystemAtLocation` "/Game/InfiniteMatrix/Blueprints/Projectile_Collision.Projectile_Collision" (`self.K2_GetActorLocation`))
      (`self.K2_DestroyActor`))
    (:`CastFailed`
      (cast `/Game/InfiniteMatrix/Blueprints/BP_Enemy` OtherActor)
      (`NiagaraFunctionLibrary.SpawnSystemAtLocation` "/Game/InfiniteMatrix/Blueprints/explosion.explosion" (`self.K2_GetActorLocation`))
      (`self.K2_DestroyActor` OtherActor)
      (`self.K2_DestroyActor`)
      (bind _returnvalue (`GameplayStatics.GetActorOfClass` "/Game/InfiniteMatrix/Blueprints/BP_Player.BP_Player_C"))
      (set `/Game/InfiniteMatrix/Blueprints/BP_Player.UserScore` (+ 5 (`/Game/InfiniteMatrix/Blueprints/BP_Player.UserScore` _returnvalue)) _returnvalue))))

(event `self.Sphere.OnComponentHit`
  (params (HitComponent :type "PrimitiveComponent Object Reference") (OtherActor :type "Actor Object Reference") (OtherComp :type "PrimitiveComponent Object Reference") (NormalImpulse :type "Vector Structure") (Hit :type "HitResult Structure (by ref)"))
  (if (not (== OtherActor (`self.GetOwner`)))
    (`PrimitiveComponent.IgnoreActorWhenMoving` (`self.Sphere`) (`GameplayStatics.GetPlayerPawn` 0) true)))

(event `self.Box.OnComponentBeginOverlap`
  (params (OverlappedComponent :type "PrimitiveComponent Object Reference") (OtherActor :type "Actor Object Reference") (OtherComp :type "PrimitiveComponent Object Reference") (OtherBodyIndex :type Integer) (bFromSweep :type Boolean) (SweepResult :type "HitResult Structure (by ref)"))
  (if (not (== OtherActor (`self.GetOwner`)))
    (bind _ashealth_pack (cast `/Game/InfiniteMatrix/Blueprints/HealthPack` OtherActor))
    (`NiagaraFunctionLibrary.SpawnSystemAtLocation` "/Game/InfiniteMatrix/Blueprints/explosion.explosion" (`self.K2_GetActorLocation`))
    (`self.K2_DestroyActor` _ashealth_pack)
    (`self.K2_DestroyActor`)))

(fn `UserConstructionScript`)