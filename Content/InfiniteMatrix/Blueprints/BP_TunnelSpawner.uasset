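; BP_TunnelSpawner builds a chain of BP_Tunnel segments, populated with health packs and enemies.
; On BeginPlay it clears existing tunnels and health packs, then spawns three segments starting at the player pawn.
; Each segment gets a spawner reference and a randomized wall, and later ones attach at the newest segment's SpawnPoint.
; Each attached segment adds a HealthPack and BP_Enemy, randomly offset in X/Y from its SpawnPoint, with Z randomized around world zero.
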(event `self.ReceiveBeginPlay`
  (`self.SpawnInitialTunnel`))

(fn `SpawnEnemy`
  (bind (_returnvalue_x _returnvalue_y) (`KismetMathLibrary.BreakVector` (`SceneComponent.K2_GetComponentLocation` (`/Game/InfiniteMatrix/Blueprints/BP_Tunnel.SpawnPoint` (`self.Newest Tunnel`)))))
  (`|SpawnActorFromClass` "/Game/InfiniteMatrix/Blueprints/BP_Enemy.BP_Enemy_C" (`KismetMathLibrary.Conv_VectorToTransform` (`KismetMathLibrary.MakeVector` (+ _returnvalue_x (`KismetMathLibrary.RandomIntegerInRange` 200 2300)) (+ _returnvalue_y (`KismetMathLibrary.RandomIntegerInRange` -200 200)) (`KismetMathLibrary.Conv_IntToDouble` (+ (`KismetMathLibrary.RandomIntegerInRange` -200 200) 0)))) "Undefined" "MultiplyWithRoot" null null))

(fn `SpawnHealth`
  (bind (_returnvalue_x _returnvalue_y) (`KismetMathLibrary.BreakVector` (`SceneComponent.K2_GetComponentLocation` (`/Game/InfiniteMatrix/Blueprints/BP_Tunnel.SpawnPoint` (`self.Newest Tunnel`)))))
  (`|SpawnActorFromClass` "/Game/InfiniteMatrix/Blueprints/HealthPack.HealthPack_C" (`KismetMathLibrary.MakeTransform` (`KismetMathLibrary.MakeVector` (+ _returnvalue_x (`KismetMathLibrary.RandomIntegerInRange` 200 2300)) (+ _returnvalue_y (`KismetMathLibrary.RandomIntegerInRange` -300 300)) (`KismetMathLibrary.Conv_IntToDouble` (+ (`KismetMathLibrary.RandomIntegerInRange` -300 300) 0)))) "Undefined" "MultiplyWithRoot" null null))

(fn `SpawnInitialTunnel`
  (`|ExecutionSequence`
    (:`then_0`
      (bind _outactors (`GameplayStatics.GetAllActorsOfClass` "/Game/InfiniteMatrix/Blueprints/BP_Tunnel.BP_Tunnel_C"))
      (for _array_element _outactors
        (`self.K2_DestroyActor` _array_element)
        (bind _outactors_2 (`GameplayStatics.GetAllActorsOfClass` "/Game/InfiniteMatrix/Blueprints/HealthPack.HealthPack_C"))
        (for _array_element_2 _outactors_2
          (`self.K2_DestroyActor` _array_element_2))))
    (:`then_1`
      (for _ (range 3)
        (`/Engine/EditorBlueprintResources/StandardMacros.IsValid` (`self.Newest Tunnel`)
          (:`Is Valid`
            (`self.SpawnTunnelAtSpawnPoint`))
          (:`Is Not Valid`
            (`self.TunnelSpawn` (`self.K2_GetActorLocation` (`GameplayStatics.GetPlayerPawn` 0)))))))))

(fn `SpawnTunnelAtSpawnPoint`
  (`self.TunnelSpawn` (`SceneComponent.K2_GetComponentLocation` (`/Game/InfiniteMatrix/Blueprints/BP_Tunnel.SpawnPoint` (`self.Newest Tunnel`))))
  (`self.SpawnHealth`)
  (`self.SpawnEnemy`))

(fn `TunnelSpawn`
  (params (SpawnLocation :type "Vector Structure"))
  (bind _returnvalue (`|SpawnActorFromClass` "/Game/InfiniteMatrix/Blueprints/BP_Tunnel.BP_Tunnel_C" (`KismetMathLibrary.MakeTransform` SpawnLocation) "Undefined" "MultiplyWithRoot" null null))
  (bind _output_get (set `self.Newest Tunnel` _returnvalue))
  (set `/Game/InfiniteMatrix/Blueprints/BP_Tunnel.TunnelSpawner` self _output_get)
  (`/Game/InfiniteMatrix/Blueprints/BP_Tunnel.RandomizeWall` _output_get))

(fn `UserConstructionScript`)